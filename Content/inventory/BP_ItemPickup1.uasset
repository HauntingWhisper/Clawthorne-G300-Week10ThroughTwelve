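; BP_ItemPickup1 is a world pickup that gives an inventory item to the player on touch.
; The construction script sets the static mesh from the Item's mesh.
; When a BP_ThirdPersonCharacter overlaps it and Item is valid, it adds the Item and Amount to the inventory through MeleeInstance, the game instance, then destroys itself.
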(event `self.ReceiveActorBeginOverlap`
  (params (OtherActor :type "Actor Object Reference"))
  (`self.item`
    (:`then`
      (cast `/Game/ThirdPerson/Blueprints/BP_ThirdPersonCharacter` OtherActor)
      (bind _asmelee_instance (cast `/Game/inventory/MeleeInstance` (`GameplayStatics.GetGameInstance`)))
      (`/Game/inventory/MeleeInstance.Add Item To Inventory` _asmelee_instance (`self.item`) (`self.amount`))
      (`self.K2_DestroyActor`))
    (:`else`)))

(fn `UserConstructionScript`
  (bind _item (`self.item`)
    (:`then`
      (`StaticMeshComponent.SetStaticMesh` (`self.StaticMesh`) (`/Game/inventory/DA_Item.mesh` _item)))
    (:`else`)))