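; BP_InventoryChecker is an actor that checks whether the player carries a specified item when the third-person character overlaps it.
; On overlap it casts to the player character, then queries the MeleeInstance game instance for ItemToCheck.
; If the item is present, it removes one from the inventory and prints the Riddle text to screen.
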(event `self.ReceiveActorBeginOverlap`
  (params (OtherActor :type "Actor Object Reference"))
  (`/Engine/EditorBlueprintResources/StandardMacros.IsValid` OtherActor
    (:`Is Valid`
      (cast `/Game/ThirdPerson/Blueprints/BP_ThirdPersonCharacter` OtherActor)
      (bind _asmelee_instance (cast `/Game/inventory/MeleeInstance` (`GameplayStatics.GetGameInstance`)))
      (bind _item_is_in_inventory (`/Game/inventory/MeleeInstance.Is Item In Inventory` _asmelee_instance (`self.Item To Check`) false))
      (if _item_is_in_inventory
        (`/Game/inventory/MeleeInstance.Remove Item From Inventory` _asmelee_instance (`self.Item To Check`) 1)
        (`KismetSystemLibrary.PrintString` (`self.Riddle`))))))

(fn `UserConstructionScript`)